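; Game mode for a classic alien shooter that tracks score, alien count and player lives.
; On BeginPlay it binds to each alien's death trigger, and each death removes that alien by column and row, adds score and decrements the count.
; RespawnPlayer deducts a life and, unless none remain, spawns the same pawn class at a player start after a delay, possesses it and updates the spaceship controller.
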(event `self.ReceiveBeginPlay`
  (for _array_element (`self.Aliens`)
    (add `Alien.AlienDeathTrigger` _array_element (delegate `AlienDeath`))))

(event `AlienDeath`
  (params (col :type Byte) (row :type Byte) (score :type Byte))
  (`self.RemoveAlien` col row)
  (set `self.Score` (+ score (`self.Score`)))
  (set `self.AlienCount` (- (`self.AlienCount`) 1)))

(event `Respawn Player`
  (params (Player :type "Pawn Object Reference"))
  (bind _returnvalue (`GameplayStatics.GetPlayerController` 0))
  (bind _output_get (set `self.PlayerLife` (- (`self.PlayerLife`) 1)))
  (if (!= _output_get 0)
    (`KismetSystemLibrary.Delay` 1.0)
    (bind _returnvalue_2 (`|SpawnActorFromClass` (`GameplayStatics.GetObjectClass` Player) (`self.GetTransform` (`self.K2_FindPlayerStart` null)) "Undefined" "MultiplyWithRoot" null null))
    (`Controller.Possess` _returnvalue _returnvalue_2)
    (bind _asplayer_spaceship_controller (cast `PlayerSpaceshipController` _returnvalue))
    (bind _asbp_player (cast `/Game/Blueprint/BP_Player` _returnvalue_2))
    (`PlayerSpaceshipController.UpdatePossessedPawn` _asplayer_spaceship_controller _asbp_player)))

(event `self.ReceiveTick`
  (params (DeltaSeconds :type "Float (single-precision)")))

(fn `UserConstructionScript`)