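; Player actor for a classic-style shooter that fires projectiles and dies when shot.
; Shoot input spawns a Projectile at an offset and blocks further shots until it is destroyed, allowing only one live shot at a time.
; A Projectile hitting the mesh destroys the player.
; On destruction, it asks BP_ClassicGameMode to respawn the player.
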(event `InputAction|Shoot`
  (params (Key :type "Key Structure"))
  (:`Pressed`
    (if (`self.CanShoot`)
      (bind _returnvalue (`|SpawnActorFromClass` (`self.Projectile`) (`KismetMathLibrary.Conv_VectorToTransform` (+ (`self.K2_GetActorLocation` self) (`self.ProjectileOffset`))) "Undefined" "MultiplyWithRoot" null null))
      (set `self.CanShoot` false)
      (add `self.OnDestroyed` _returnvalue (delegate `OnDestroyed_Event`)))))

(event `OnDestroyed_Event` :!signature `self.OnDestroyed`
  (params (DestroyedActor :type "Actor Object Reference"))
  (set `self.CanShoot` true))

(event `self.Mesh.OnComponentHit`
  (params (HitComponent :type "PrimitiveComponent Object Reference") (OtherActor :type "Actor Object Reference") (OtherComp :type "PrimitiveComponent Object Reference") (NormalImpulse :type "Vector Structure") (Hit :type "HitResult Structure (by ref)"))
  (cast `Projectile` OtherActor)
  (`self.K2_DestroyActor`))

(event `self.ReceiveDestroyed`
  (bind _asbp_classic_game_mode (cast `/Game/Blueprint/BP_ClassicGameMode` (`GameplayStatics.GetGameMode`)))
  (`/Game/Blueprint/BP_ClassicGameMode.Respawn Player` _asbp_classic_game_mode self))

(fn `UserConstructionScript`)